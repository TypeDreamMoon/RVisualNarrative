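; BP_Dialogue_NPC is an NPC actor that starts a dialogue when the player character enters its trigger box.
; On Box begin overlap, it casts to BP_ThirdPersonCharacter and adds a dialogue component at runtime if none is valid yet, caching it for later overlaps.
; It then passes that component's dialogue manager to the character's StartDialogue.
; Leaving the box does nothing.
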(event OnComponentBeginOverlap(Box)
  (params (OverlappedComponent :type Primitive%20Component%20Object%20Reference) (OtherActor :type Actor%20Object%20Reference) (OtherComp :type Primitive%20Component%20Object%20Reference) (OtherBodyIndex :type Integer) (bFromSweep :type Boolean) (SweepResult :type Hit%20Result%20Structure%20%28by%20ref%29))
  (bind _asbp_third_person_character (Utilities|Casting|CastToBP_ThirdPersonCharacter OtherActor))
  (Variables|Default|SetAs%20BP%20Third%20Person%20Character _asbp_third_person_character)
  (Utilities|IsValid (Variables|Default|GetRVNComponentObj)
    (:Is%20Valid
      _)
    (:Is%20Not%20Valid
      (bind _returnvalue (Game|AddComponentbyClass (Variables|Default|GetDialogueComp)))
      (Variables|Default|SetRVNComponentObj _returnvalue)))
  (bind _returnvalue_2 (Class|RVNComponent|GetDialogueManager (Variables|Default|GetRVNComponentObj)))
  (Default|StartDialogue (Variables|Default|GetAs%20BP%20Third%20Person%20Character) _returnvalue_2))

(event OnComponentEndOverlap(Box)
  (params (OverlappedComponent :type Primitive%20Component%20Object%20Reference) (OtherActor :type Actor%20Object%20Reference) (OtherComp :type Primitive%20Component%20Object%20Reference) (OtherBodyIndex :type Integer)))

(event EventBeginPlay)

(event Collision|EventActorBeginOverlap
  (params (OtherActor :type Actor%20Object%20Reference)))

(event EventTick
  (params (DeltaSeconds :type Float%20%28single-precision%29)))

(fn ConstructionScript)