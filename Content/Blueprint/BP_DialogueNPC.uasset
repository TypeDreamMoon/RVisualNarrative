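; BP_DialogueNPC is a dialogue NPC that opens a dialogue UI as soon as play begins.
; It adds a dialogue component at runtime, then hands that component's dialogue manager to a new main dialogue widget.
; The widget starts hidden so stray root information is not seen, and input switches to game and UI.
; When the manager reports completion, input returns to game only, with the mouse cursor left visible.
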(event Custom|OnDialogueEnd
  (bind _returnvalue (Game|GetPlayerController 0))
  (Variables|/Script/Engine.PlayerController|SetbShowMouseCursor _returnvalue true)
  (Input|SetInputModeGameOnly _returnvalue))

(event EventBeginPlay
  (bind _returnvalue (Game|GetPlayerController 0))
  (bind _returnvalue_2 (Game|AddComponentbyClass (Variables|Default|GetDialogueComp)))
  (Variables|Default|SetDialogueCompObj _returnvalue_2)
  (bind _returnvalue_3 (Class|RVNComponent|GetDialogueManager (Variables|Default|GetDialogueCompObj)))
  (EventDispatchers|BindEventtoOnDialogueCompleted _returnvalue_3 (delegate Custom|OnDialogueEnd))
  (Variables|/Script/Engine.PlayerController|SetbShowMouseCursor _returnvalue true)
  (bind _returnvalue_4 (UserInterface|CreateWidget (Variables|Default|GetMainDialogueWidget) _returnvalue))
  (bind _output_get (Variables|Default|SetMainDialogueWidgetObj _returnvalue_4))
  ;[1 1 1] 防止看见无用的Root信息
  (Widget|SetVisibility _output_get "Hidden")
  (UserInterface|Viewport|AddtoViewport _output_get 0)
  (Input|SetInputModeGameandUI _returnvalue _output_get "DoNotLock" true)
  (Default|StartDialogue _output_get _returnvalue_3))

(fn ConstructionScript)